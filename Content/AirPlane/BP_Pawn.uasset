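; Player airplane pawn that flies forward constantly and fires rockets.
; Tick feeds movement input along the forward vector, with Boost switching between full and half throttle, while Roll and Pitch axes apply clamped, frame-rate-independent world rotations.
; Shoot spawns BP_Rocket at the Arrow transform with the pawn as owner.
; BeginPlay registers the Left and Right components in the BPActorCompo component's SceneComponent array.
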(event `self.ReceiveBeginPlay`
  (`KismetArrayLibrary.Array_Add` (`/Game/AirPlane/BP_ActorCompo.SceneComponent` (`self.BP_ActorCompo`)) (`self.Left`))
  (`KismetArrayLibrary.Array_Add` (`/Game/AirPlane/BP_ActorCompo.SceneComponent` (`self.BP_ActorCompo`)) (`self.Right`)))

(event `self.ReceiveTick`
  (params (DeltaSeconds :type "Float (single-precision)"))
  (`self.AddMovementInput` (`self.GetActorForwardVector`) (`self.Scale Value`)))

(event `InputAxis|Roll`
  (params (AxisValue :type "Float (single-precision)"))
  (`self.K2_AddActorWorldRotation` (`KismetMathLibrary.MakeRotator` (* (`KismetMathLibrary.FClamp` AxisValue -1.0) (`GameplayStatics.GetWorldDeltaSeconds`) 60.0))))

(event `InputAction|Boost`
  (params (Key :type "Key Structure"))
  (:`Pressed`
    (set `self.Scale Value` 1.0))
  (:`Released`
    (set `self.Scale Value` 0.5)))

(event `InputAxis|Pitch`
  (params (AxisValue :type "Float (single-precision)"))
  (`self.K2_AddActorWorldRotation` (`KismetMathLibrary.MakeRotator` 0.0 (* (`KismetMathLibrary.FClamp` AxisValue -1.0) (`GameplayStatics.GetWorldDeltaSeconds`) 60.0))))

(event `InputAction|Shoot`
  (params (Key :type "Key Structure"))
  (:`Pressed`
    (`|SpawnActorFromClass` "/Game/AirPlane/BP_Rocket.BP_Rocket_C" (`SceneComponent.K2_GetComponentToWorld` (`self.Arrow`)) "Undefined" "MultiplyWithRoot" self null)))

(fn `UserConstructionScript`)